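; BP_Digimon is a combat unit for turn-based Digimon battles, with data-driven stats, a mesh and a health/mana bar.
; SetupVariables loads model, AnimBP, stats, skills and evolutions from DT_DigimonSkills by name; Digivolve reruns it with the new form, resetting health and mana.
; Action and death events message the AnimInstance, and player-controlled units advance BP_CombatManager's turn after a delay.
; Tick refreshes the bar and rotates it toward the camera.
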(event `self.ReceiveBeginPlay`
  ;[1 1 1] Setup Variables and Start Combat Manager
  (`self.SetupVariables` (`self.DigimonName`)))

(event `DigimonAction`
  (params (Skill :type "/Game/MyGame/Enums/Enum_Actions Enum" :default "NewEnumerator0"))
  (bind _output_get (set `self.SkillTriggered` Skill))
  (message `/Game/MyGame/Blueprints/BPI_Animation.TriggerAnimation` (`self.AnimInstance`) _output_get)
  (if (`|EnumEquality` (`self.ControlledBy`) "NewEnumerator0")
    (`KismetSystemLibrary.Delay` 2.0)
    (bind _returnvalue (`GameplayStatics.GetActorOfClass` "/Game/MyGame/Blueprints/BP_CombatManager.BP_CombatManager_C"))
    (`/Game/MyGame/Blueprints/BP_CombatManager.TriggerNextTurn` _returnvalue)))

(event `DeathAnim`
  (message `/Game/MyGame/Blueprints/BPI_Animation.TriggerDeath` (`self.AnimInstance`)))

(event `Digivolve`
  (params (EvolutionType :type Name))
  (`self.SetupVariables` EvolutionType))

(event `self.ReceiveTick`
  (params (DeltaSeconds :type "Float (single-precision)"))
  (bind _healthbar (`self.HealthBar`))
  (bind _aswidget_health_bar (cast `/Game/MyGame/UI/Widget_HealthBar` (`WidgetComponent.GetWidget` (`self.HealthBar`))))
  (`ProgressBar.SetPercent` (`/Game/MyGame/UI/Widget_HealthBar.Health` _aswidget_health_bar) (/ (`self.CurrentHealth`) (`KismetMathLibrary.Conv_IntToDouble` (`self.MaxHealth`))))
  (`ProgressBar.SetPercent` (`/Game/MyGame/UI/Widget_HealthBar.Mana` _aswidget_health_bar) (/ (`self.CurrentMana`) 4.0))
  (`SceneComponent.K2_SetWorldRotation` _healthbar (`KismetMathLibrary.FindLookAtRotation` (`SceneComponent.K2_GetComponentLocation` _healthbar) (`SceneComponent.K2_GetComponentLocation` (`PlayerCameraManager.TransformComponent` (`GameplayStatics.GetPlayerCameraManager` 0)))) false false))

(fn `SetupVariables`
  (params (`Digimon Name` :type Name))
  (bind _digimon (`self.Digimon`))
  (bind _returnvalue (`|GetDataTableRow` "/Game/MyGame/Enums/DT_DigimonSkills.DT_DigimonSkills" `Digimon Name`)
    (:`then`
      (`SkeletalMeshComponent.SetSkeletalMeshAsset` _digimon (`.SM_Model_34_05D71BC24ED0ADF574657B82DE68BF09` (break `/Game/MyGame/Enums/Struct_DigimonSkillData` _returnvalue)))
      (`SkeletalMeshComponent.SetAnimInstanceClass` _digimon (`.AnimationBP_44_819237F245C201C035D0A4AA97EE8DD1` (break `/Game/MyGame/Enums/Struct_DigimonSkillData` _returnvalue)))
      (set `self.Species` (break `/Game/MyGame/Enums/Struct_DigimonSkillData` _returnvalue))
      (set `self.MaxHealth` (`.DigimonHP_26_72D4FC064DD19AD257C1DB8CCBC96862` (break `/Game/MyGame/Enums/Struct_DigimonSkillData` _returnvalue)))
      (set `self.CurrentMana` 0)
      (set `self.Type` (`.DigimonType_27_474B0E7249B9BD4DDF16B7B32E456E82` (break `/Game/MyGame/Enums/Struct_DigimonSkillData` _returnvalue)))
      (set `self.DigimonRole` (`.DigimonRole_28_63E5F7014B28FDC785492984B1ECCAEB` (break `/Game/MyGame/Enums/Struct_DigimonSkillData` _returnvalue)))
      (set `self.EvolutionStage` (`.EvolutionStage_31_6F9805E643F73230110E33B3A6EA97AD` (break `/Game/MyGame/Enums/Struct_DigimonSkillData` _returnvalue)))
      (set `self.BasicDmg` (`.BasicAttackDmg_5_BC4642F14C11DDD85BD8A2B2BEC6993F` (break `/Game/MyGame/Enums/Struct_DigimonSkillData` _returnvalue)))
      (set `self.Skill1Dmg` (`.Skill1Dmg_9_127FBD4441A8004B39ADB5924F43DE7B` (break `/Game/MyGame/Enums/Struct_DigimonSkillData` _returnvalue)))
      (set `self.Skill1Mana` (`.Skill1Mana_11_CCC7BD284243A250463EDC9BC42543E6` (break `/Game/MyGame/Enums/Struct_DigimonSkillData` _returnvalue)))
      (set `self.Skill2Dmg` (`.Skill2Dmg_13_29F9C7B5400D68ECD2AD938909B86DC1` (break `/Game/MyGame/Enums/Struct_DigimonSkillData` _returnvalue)))
      (set `self.Skill2Mana` (`.Skill2Mana_15_CF9141494135054E5CB8B39E1EEE2B93` (break `/Game/MyGame/Enums/Struct_DigimonSkillData` _returnvalue)))
      (set `self.Evolution1` (`.Evolution1_53_57B8AC4D4A46CF5591990383DD2C4D1C` (break `/Game/MyGame/Enums/Struct_DigimonSkillData` _returnvalue)))
      (set `self.Evolution2` (`.Evolution2_54_A0DF6ABA46409DC7101F2392D1B4D62D` (break `/Game/MyGame/Enums/Struct_DigimonSkillData` _returnvalue)))
      (set `self.CurrentHealth` (`self.MaxHealth`))
      (set `self.CurrentMana` 0)
      (set `self.AnimInstance` (`SkeletalMeshComponent.GetAnimInstance` (`self.Digimon`)))
      (switch `/Game/MyGame/Enums/Enum_ControlledBy` (`self.ControlledBy`)
        (:`NewEnumerator0`
          (set `self.AIControllerClass` null))))))

(fn `UserConstructionScript`)